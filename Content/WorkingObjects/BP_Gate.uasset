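; BP_Gate is an actor that periodically heals and restocks ammo for a first-person character overlapping it.
; Actor begin-overlap caches the BP_FirstPersonCharacter, and the Box component's end-overlap clears that reference.
; While the reference is valid, Tick accumulates delta time and, about once per second, calls Heal on the character's BPCDamageSystem and increases its Ammo.
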(event `self.ReceiveActorBeginOverlap`
  (params (OtherActor :type "Actor Object Reference"))
  (bind _asbp_first_person_character (cast `/Game/FirstPerson/Blueprints/BP_FirstPersonCharacter` OtherActor))
  (set `self.As BP First Person Character` _asbp_first_person_character))

(event `self.Box.OnComponentEndOverlap`
  (params (OverlappedComponent :type "PrimitiveComponent Object Reference") (OtherActor :type "Actor Object Reference") (OtherComp :type "PrimitiveComponent Object Reference") (OtherBodyIndex :type Integer))
  (cast `/Game/FirstPerson/Blueprints/BP_FirstPersonCharacter` OtherActor)
  (set `self.As BP First Person Character` null))

(event `self.ReceiveTick`
  (params (DeltaSeconds :type "Float (single-precision)"))
  (bind _as_bp_first_person_character (`self.As BP First Person Character`))
  (`/Engine/EditorBlueprintResources/StandardMacros.IsValid` (`self.As BP First Person Character`)
    (:`Is Valid`
      (if (>= (`self.TimePassed`) 1.0)
        (set `self.TimePassed` 0.0)
        (`/Game/DamageSystem/BPC_DamageSystem.Heal` (`/Game/FirstPerson/Blueprints/BP_FirstPersonCharacter.BPC_DamageSystem` _as_bp_first_person_character) 10.0)
        (set `/Game/FirstPerson/Blueprints/BP_FirstPersonCharacter.Ammo` (+ (`/Game/FirstPerson/Blueprints/BP_FirstPersonCharacter.Ammo` _as_bp_first_person_character) 10.0) _as_bp_first_person_character)
        (else
          (set `self.TimePassed` (+ DeltaSeconds (`self.TimePassed`))))))))

(fn `UserConstructionScript`)