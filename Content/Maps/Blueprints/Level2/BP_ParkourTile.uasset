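; BP_ParkourTile is a Level 2 parkour tile that changes its material shine when stepped on and off.
; Box overlaps count only when the other component's name contains "CollisionCylinder", likely a character capsule.
; Overlap begin plays one timeline, and overlap end reverses a separate timeline from its end.
; Each timeline's track drives the "Shine" scalar parameter on the Tile's materials.
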(event `self.Box Collision.OnComponentBeginOverlap`
  (params (OverlappedComponent :type "PrimitiveComponent Object Reference") (OtherActor :type "Actor Object Reference") (OtherComp :type "PrimitiveComponent Object Reference") (OtherBodyIndex :type Integer) (bFromSweep :type Boolean) (SweepResult :type "HitResult Structure (by ref)"))
  (if (`KismetStringLibrary.Contains` (`KismetSystemLibrary.GetObjectName` OtherComp) "CollisionCylinder")
    (bind (_direction _newtrack_0) (`Timeline|Timeline`)
      (:`Update`
        (`MeshComponent.SetScalarParameterValueOnMaterials` (`self.Tile`) "Shine" _newtrack_0)))))

(event `self.Box Collision.OnComponentEndOverlap`
  (params (OverlappedComponent :type "PrimitiveComponent Object Reference") (OtherActor :type "Actor Object Reference") (OtherComp :type "PrimitiveComponent Object Reference") (OtherBodyIndex :type Integer))
  (if (`KismetStringLibrary.Contains` (`KismetSystemLibrary.GetObjectName` OtherComp) "CollisionCylinder")
    (bind (_direction _newtrack_0) (`Timeline|Timeline_0` :!via `ReverseFromEnd`)
      (:`Update`
        (`MeshComponent.SetScalarParameterValueOnMaterials` (`self.Tile`) "Shine" _newtrack_0)))))

(fn `UserConstructionScript`)