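; BP_WaveAfterWave is a Level3 enemy spawner that releases a set number of waves on a timer.
; BeginPlay loops while Waves remain, decrementing the count, calling SpawnWave and delaying by WaveInterval.
; SpawnWave visits five SpawnPoint entries, spawning HowManyEnemiesPerSpawnPoint actors at each.
; Each actor gets a random class from the Class array and a random X/Y offset, keeping the point's Z.
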(event `self.ReceiveBeginPlay`
  (bind _waves (`self.Waves`))
  (if (> _waves 0) :!label _label
    (`/Engine/EditorBlueprintResources/StandardMacros.DecrementInt` _waves
      (:`  `
        (`self.SpawnWave`)
        (`KismetSystemLibrary.Delay` (`self.Wave Interval`))
        (goto _label)))))

(event `SpawnWave`
  (bind _offset (`self.Offset`))
  (bind _returnvalue (`KismetMathLibrary.RandomFloatInRange` (* _offset -1.0) _offset))
  (for _index (range 5)
    (for _ (range (`self.How many enemies per spawn point?`))
      (`|SpawnActorFromClass` (`KismetArrayLibrary.Array_Random` (`self.Class`)) (`KismetMathLibrary.MakeTransform` (`KismetMathLibrary.MakeVector` (+ (.x (`|GetArrayItem` (`self.Spawn Point`) _index)) _returnvalue) (+ (.y (`|GetArrayItem` (`self.Spawn Point`) _index)) _returnvalue) (.z (`|GetArrayItem` (`self.Spawn Point`) _index)))) "Undefined" "MultiplyWithRoot" null null))))

(fn `UserConstructionScript`)