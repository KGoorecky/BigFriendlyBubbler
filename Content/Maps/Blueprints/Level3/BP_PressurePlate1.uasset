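; Level 3 pressure plate that plays a one-shot cinematic reveal, then starts an enemy wave encounter.
; Overlap destroys the trigger box and animates the plane's Shine before removing it.
; The view blends to a rotating Camera1 while delayed sequence branches stagger spotlights and temporary skeletal meshes facing Start.
; It then fires LIGHTSON, restores the saved view, fires SHOWMERCY, spawns BP_WaveAfterWave and removes the temporary meshes.
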(event `self.Box.OnComponentBeginOverlap`
  (params (OverlappedComponent :type "PrimitiveComponent Object Reference") (OtherActor :type "Actor Object Reference") (OtherComp :type "PrimitiveComponent Object Reference") (OtherBodyIndex :type Integer) (bFromSweep :type Boolean) (SweepResult :type "HitResult Structure (by ref)"))
  (bind _loc1 (`self.Loc1`))
  (bind _loc2 (`self.Loc2`))
  (bind _loc3 (`self.Loc3`))
  (bind _loc4 (`self.Loc4`))
  (bind _spotlight1 (`self.SpotLight1`))
  (bind _returnvalue (- _loc4 (0.0 0.0 500.0)))
  (bind _returnvalue_2 (- _loc1 (0.0 0.0 500.0)))
  (bind _returnvalue_3 (- _loc2 (0.0 0.0 500.0)))
  (bind _returnvalue_4 (- _loc3 (0.0 0.0 500.0)))
  (bind (_returnvalue_roll _returnvalue_pitch _returnvalue_yaw) (`KismetMathLibrary.BreakRotator` (`KismetMathLibrary.FindLookAtRotation` _returnvalue (`self.Start`))))
  (bind (_returnvalue_roll_2 _returnvalue_pitch_2 _returnvalue_yaw_2) (`KismetMathLibrary.BreakRotator` (`KismetMathLibrary.FindLookAtRotation` _returnvalue_2 (`self.Start`))))
  (bind (_returnvalue_roll_3 _returnvalue_pitch_3 _returnvalue_yaw_3) (`KismetMathLibrary.BreakRotator` (`KismetMathLibrary.FindLookAtRotation` _returnvalue_3 (`self.Start`))))
  (bind (_returnvalue_roll_4 _returnvalue_pitch_4 _returnvalue_yaw_4) (`KismetMathLibrary.BreakRotator` (`KismetMathLibrary.FindLookAtRotation` _returnvalue_4 (`self.Start`))))
  (set `self.PlayerCamera` (`Controller.GetViewTarget` (`GameplayStatics.GetPlayerController` 0)))
  (`ActorComponent.K2_DestroyComponent` (`self.Box`))
  (bind (_direction _newtrack_0) (`Timeline|Timeline` :!via `PlayFromStart`)
    (:`Update`
      (`MeshComponent.SetScalarParameterValueOnMaterials` (`self.Plane`) "Shine" _newtrack_0))
    (:`Finished`
      (`ActorComponent.K2_DestroyComponent` (`self.Plane`))
      (`KismetSystemLibrary.Delay` 0.1)
      (`SceneComponent.SetVisibility` _spotlight1 true false)
      (`SceneComponent.K2_SetWorldTransform` _spotlight1 (`KismetMathLibrary.MakeTransform` (0.0 150.0 3000.0) (struct :`Pitch` -90.0)) false false)
      (`|ExecutionSequence`
        (:`then_0`
          (bind _returnvalue_5 (`GameplayStatics.GetActorOfClass` "/Game/Maps/Blueprints/Level3/camera1.camera1_C"))
          (`PlayerController.SetViewTargetWithBlend` (`GameplayStatics.GetPlayerController` 0) _returnvalue_5 2.0 "VTBlend_Linear" 2.0 false)
          (`ActorComponent.Activate` (`/Game/Maps/Blueprints/Level3/camera1.Camera` _returnvalue_5) false)
          (`AddComponent|NODE_AddRotatingMovementComponent-0` :`self` _returnvalue_5))
        (:`then_1`
          (`KismetSystemLibrary.Delay` 4.0)
          (`SceneComponent.K2_SetWorldTransform` (`self.SpotLight2`) (`KismetMathLibrary.MakeTransform` _loc1 (struct :`Pitch` -90.0)) false false)
          (bind _returnvalue_6 (`AddComponent|NODE_AddSkeletalMeshComponent-0`))
          (`SceneComponent.K2_SetWorldLocationAndRotation` _returnvalue_6 _returnvalue_2 (`KismetMathLibrary.MakeRotator` 0.0 0.0 _returnvalue_yaw_2) false false))
        (:`then_2`
          (`KismetSystemLibrary.Delay` 5.0)
          (`SceneComponent.K2_SetWorldTransform` (`self.SpotLight3`) (`KismetMathLibrary.MakeTransform` _loc2 (struct :`Pitch` -90.0)) false false)
          (bind _returnvalue_7 (`AddComponent|NODE_AddSkeletalMeshComponent-1`))
          (`SceneComponent.K2_SetWorldLocationAndRotation` _returnvalue_7 _returnvalue_3 (`KismetMathLibrary.MakeRotator` 0.0 0.0 _returnvalue_yaw_3) false false))
        (:`then_3`
          (`KismetSystemLibrary.Delay` 6.0)
          (`SceneComponent.K2_SetWorldTransform` (`self.SpotLight4`) (`KismetMathLibrary.MakeTransform` _loc3 (struct :`Pitch` -90.0)) false false)
          (bind _returnvalue_8 (`AddComponent|NODE_AddSkeletalMeshComponent-2`))
          (`SceneComponent.K2_SetWorldLocationAndRotation` _returnvalue_8 _returnvalue_4 (`KismetMathLibrary.MakeRotator` 0.0 0.0 _returnvalue_yaw_4) false false))
        (:`then_4`
          (`KismetSystemLibrary.Delay` 7.0)
          (`SceneComponent.K2_SetWorldTransform` (`self.SpotLight5`) (`KismetMathLibrary.MakeTransform` _loc4 (struct :`Pitch` -90.0)) false false)
          (bind _returnvalue_9 (`AddComponent|NODE_AddSkeletalMeshComponent-3`))
          (`SceneComponent.K2_SetWorldLocationAndRotation` _returnvalue_9 _returnvalue (`KismetMathLibrary.MakeRotator` 0.0 0.0 _returnvalue_yaw) false false)
          (`KismetSystemLibrary.Delay` 1.0)
          (`self.LIGHTSON`)
          (`PlayerController.SetViewTargetWithBlend` (`GameplayStatics.GetPlayerController` 0) (`self.PlayerCamera`) 2.0 "VTBlend_Linear" 3.0 false)
          (`self.SHOWMERCY`)
          (`|SpawnActorFromClass` "/Game/Maps/Blueprints/Level3/BP_WaveAfterWave.BP_WaveAfterWave_C" (`KismetMathLibrary.MakeTransform` (0.0 0.0 0.0)) "Undefined" "MultiplyWithRoot" null (`self.Spawn Point`) 2 4 15.0 null)
          (`ActorComponent.K2_DestroyComponent` _returnvalue_9)
          (`ActorComponent.K2_DestroyComponent` _returnvalue_8)
          (`ActorComponent.K2_DestroyComponent` _returnvalue_7)
          (`ActorComponent.K2_DestroyComponent` _returnvalue_6))))))

(fn `UserConstructionScript`)