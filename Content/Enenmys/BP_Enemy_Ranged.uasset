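; BP_Enemy_Ranged is a ranged enemy that fires a bullet and reacts to damage and death.
; Attack plays a gunshot and firing montage, spawns the projectile ahead of the actor when the montage completes, then signals attack end, which also fires on interruption.
; Damage component events play a hit sound or, on death, hide the health bar, disable capsule collision, and play a dance montage before destroying the actor.
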(event `self.Attack`
  (bind (_returnvalue_x _returnvalue_y _returnvalue_z) (`KismetMathLibrary.BreakVector` (+ (* (`KismetMathLibrary.Normal` (`self.GetActorForwardVector`)) 50.0) (`self.K2_GetActorLocation`))))
  (`GameplayStatics.PlaySoundAtLocation` "/Game/EnemiesAssets/EnemiesModels/robor/shotGun.shotGun" (`self.K2_GetActorLocation`) (struct) 1.0 1.0 0.0 null null null null)
  (`|PlayMontage` (`self.Mesh`) "/Game/EnemiesAssets/EnemiesModels/robor/firing_rifle_Montage.firing_rifle_Montage"
    (:`OnCompleted`
      (`|SpawnActorFromClass` "/Game/FirstPerson/Blueprints/BP_Bullet_Mati_Oponent.BP_Bullet_Mati_Oponent_C" (`KismetMathLibrary.MakeTransform` (`KismetMathLibrary.MakeVector` _returnvalue_x _returnvalue_y (+ _returnvalue_z 50.0)) (`self.K2_GetActorRotation`)) "Undefined" "MultiplyWithRoot" null null))
    (:`OnInterrupted`
      _))
  (`self.OnAttackEnd`))

(event `self.BPC_DamageSystem.OnDeath`
  (`SceneComponent.SetVisibility` (`self.HealthBar`) false false)
  (`PrimitiveComponent.SetCollisionEnabled` (`self.CapsuleComponent`) "NoCollision")
  (`|PlayMontage` (`self.Mesh`) "/Game/EnemiesAssets/EnemiesModels/robor/Wave_Hip_Hop_Dance_Montage_EPIC.Wave_Hip_Hop_Dance_Montage_EPIC"
    (:`OnCompleted`
      (`self.K2_DestroyActor`))))

(event `self.BPC_DamageSystem.OnDamageResponse`
  (params (DamageResponse :type "/Game/DamageSystem/E_DamageResponses Enum" :default "NewEnumerator0"))
  (`GameplayStatics.PlaySoundAtLocation` "/Game/EnemiesAssets/EnemiesModels/robor/metalBeastHitSound.metalBeastHitSound" (`self.K2_GetActorLocation`) (struct) 1.0 1.0 0.0 null null null null))

(fn `UserConstructionScript`
  (`parent.UserConstructionScript`))