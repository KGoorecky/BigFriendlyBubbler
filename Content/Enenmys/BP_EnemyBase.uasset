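; Base enemy character that exposes health, damage, patrol route and movement speed functions, driven by an AIC_Enemy_Base AI controller.
; BPC_DamageSystem handles health and damage, while a health bar widget stays hidden until the controller signals to show it.
; Damage responses stop movement, freeze the AI and play a hit montage before resuming attack.
; Attack plays a montage and signals its end; TakeDamage also feeds pre-hit health into Niagara parameters.
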(event `self.ReceiveBeginPlay`
  (bind _asaic_enemy_base (cast `/Game/Enenmys/AI/AIC_Enemy_Base` (`AIBlueprintHelperLibrary.GetAIController` self)))
  (set `self.As AIC Enemy Base` _asaic_enemy_base)
  (bind _returnvalue (`|CreateWidget` "/Game/DamageSystem/W_HealthBar.W_HealthBar_C" null self))
  (`WidgetComponent.SetWidget` (`self.HealthBar`) _returnvalue)
  (`SceneComponent.SetVisibility` (`self.HealthBar`) false false)
  (add `/Game/DamageSystem/BPC_DamageSystem.OnDamageResponse` (`self.BPC_DamageSystem`) (`|CreateDelegate` :!event `Hit Response`))
  (add `/Game/Enenmys/AI/AIC_Enemy_Base.ShowHealthBar` (`self.As AIC Enemy Base`) (delegate `ShowWidget`)))

(event `ShowWidget`
  (`SceneComponent.SetVisibility` (`self.HealthBar`) true false))

(event `Attack`
  (`KismetSystemLibrary.PrintString` "attack")
  (`|PlayMontage` (`self.Mesh`) "/Game/Characters/Mannequins/Animations/Manny/AM_MannyAttack.AM_MannyAttack"
    (:`OnCompleted`
      _)
    (:`OnInterrupted`
      _))
  (`self.OnAttackEnd`))

(event `self.BPC_DamageSystem.OnDeath`)

(event `Hit Response`
  (params (DamageResponse :type "/Game/DamageSystem/E_DamageResponses Enum" :default "NewEnumerator0"))
  (`MovementComponent.StopMovementImmediately` (`self.CharacterMovement`))
  (`/Game/Enenmys/AI/AIC_Enemy_Base.Set State As Frozen` (`self.As AIC Enemy Base`))
  (`|PlayMontage` (`self.Mesh`) (`self.Hit Reaction Montage to Play`)
    (:`OnCompleted`
      _)
    (:`OnInterrupted`
      _))
  (`/Game/Enenmys/AI/AIC_Enemy_Base.Set State As Attacking` (`self.As AIC Enemy Base`) null true))

(fn `GetCurretnHealth`
  (returns (Health :type "Float (double-precision)"))
  (return (`/Game/DamageSystem/BPC_DamageSystem.Health` (`self.BPC_DamageSystem`))))

(fn `GetMaxHealth`
  (returns (MaxHealth :type "Float (double-precision)"))
  (return (`/Game/DamageSystem/BPC_DamageSystem.MaxHealth` (`self.BPC_DamageSystem`))))

(fn `GetPatrolRoute`
  (returns (PatrolRoute :type "/Game/Enenmys/AI/BP_PatrollRoute Object Reference"))
  (return (`self.PatrolRoute`)))

(fn `Heal`
  (params (Amount :type "Float (double-precision)"))
  (returns (NewHealth :type "Float (double-precision)"))
  (bind _newhealth (`/Game/DamageSystem/BPC_DamageSystem.Heal` (`self.BPC_DamageSystem`) Amount))
  (return _newhealth))

(fn `IsDead`
  (returns (IsDead :type Boolean))
  (return (`/Game/DamageSystem/BPC_DamageSystem.IsDead` (`self.BPC_DamageSystem`))))

(fn `SetMovmentSpeed`
  (params (Speed :type "/Game/Enenmys/AI/Enums/E_MovmentSpeed Enum" :default "NewEnumerator0"))
  (returns (SpeedValue :type "Float (double-precision)"))
  (bind _output_get (set `CharacterMovementComponent.MaxWalkSpeed` (select `/Game/Enenmys/AI/Enums/E_MovmentSpeed` Speed :`NewEnumerator1` 100.0 :`NewEnumerator2` 300.0 :`NewEnumerator3` 500.0 :!type "Float (single-precision)") (`self.CharacterMovement`)))
  (return _output_get))

(fn `TakeDamage`
  (params (`Damage Info` :type "/Game/DamageSystem/S_DamageInfo Structure"))
  (returns (WasDamaged :type Boolean))
  (bind _niagara (`self.Niagara`))
  (bind _bpc_damagesystem (`self.BPC_DamageSystem`))
  (bind _health (`/Game/DamageSystem/BPC_DamageSystem.Health` _bpc_damagesystem))
  (`NiagaraComponent.SetVariableFloat` _niagara "aa" _health)
  (`NiagaraComponent.SetVariableFloat` _niagara "kolor" (/ (- _health 0.3) (- (`/Game/DamageSystem/BPC_DamageSystem.MaxHealth` _bpc_damagesystem) 0.3)))
  (bind _damaged (`/Game/DamageSystem/BPC_DamageSystem.Take Damage` (`self.BPC_DamageSystem`) `Damage Info`))
  (return _damaged))

(fn `UserConstructionScript`)