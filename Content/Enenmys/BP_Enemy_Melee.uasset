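; Melee enemy character that strikes the player at close range and reacts to damage and death through a damage system component.
; Attack plays a sound and montage, uses a montage notify to sphere-trace forward and damage only the player, then signals attack end on completion or interruption.
; Damage plays a sound, while death hides the health bar, disables capsule collision and destroys the actor after its montage.
; SetMovmentSpeed maps movement states to walk speeds.
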(event `self.Attack`
  (bind _returnvalue (`self.K2_GetActorLocation`))
  (`GameplayStatics.PlaySoundAtLocation` "/Game/EnemiesAssets/EnemiesModels/Klaun/jonklerProvokation.jonklerProvokation" (`self.K2_GetActorLocation`) (struct) 1.0 1.0 0.0 null null null null)
  (bind _notifyname (`|PlayMontage` (`self.Mesh`) "/Game/EnemiesAssets/EnemiesModels/Klaun/Anims/standing_melee_attack_downward_Montage.standing_melee_attack_downward_Montage")
    (:`then`
      (set `/Game/DamageSystem/BPC_DamageSystem.IsInteruptible` false (`self.BPC_DamageSystem`)))
    (:`OnCompleted`
      (`self.OnAttackEnd` :!label _label)
      (set `/Game/DamageSystem/BPC_DamageSystem.IsInteruptible` false (`self.BPC_DamageSystem`)))
    (:`OnInterrupted`
      (goto _label))
    (:`OnNotifyBegin`
      (switch `name` _notifyname
        (:`Slash`
          (bind (_outhit _returnvalue_2) (`KismetSystemLibrary.SphereTraceSingleForObjects` :`Start` _returnvalue :`End` (+ _returnvalue (* (`self.GetActorForwardVector`) 200.0)) :`Radius` 20.0 :`ObjectTypes` (`|MakeArray` "ObjectTypeQuery3" :!type "EObjectTypeQuery Enum") :`DrawDebugType` "ForDuration"))
          (if _returnvalue_2
            (bind (_bblockinghit _binitialoverlap _time _distance _location _impactpoint _normal _impactnormal _physmat _hitactor) (`GameplayStatics.BreakHitResult` _outhit))
            (if (== _hitactor (`GameplayStatics.GetPlayerCharacter` 0))
              (message `/Game/DamageSystem/BPI_Damgeable.TakeDamage` _hitactor (make `/Game/DamageSystem/S_DamageInfo` 20.0)))))))))

(event `self.BPC_DamageSystem.OnDeath`
  (`SceneComponent.SetVisibility` (`self.HealthBar`) false false)
  (`PrimitiveComponent.SetCollisionEnabled` (`self.CapsuleComponent`) "NoCollision")
  (`|PlayMontage` (`self.Mesh`) "/Game/EnemiesAssets/EnemiesModels/Klaun/Anims/Dribble_Klaun_Death.Dribble_Klaun_Death"
    (:`OnCompleted`
      (`self.K2_DestroyActor`))))

(event `self.BPC_DamageSystem.OnDamageResponse`
  (params (DamageResponse :type "/Game/DamageSystem/E_DamageResponses Enum" :default "NewEnumerator0"))
  (`GameplayStatics.PlaySoundAtLocation` "/Game/EnemiesAssets/EnemiesModels/Klaun/shacoReference.shacoReference" (`self.K2_GetActorLocation`) (struct) 1.0 1.0 0.0 null null null null))

(fn `SetMovmentSpeed`
  (params (Speed :type "/Game/Enenmys/AI/Enums/E_MovmentSpeed Enum" :default "NewEnumerator0"))
  (returns (SpeedValue :type "Float (double-precision)"))
  (bind _output_get (set `CharacterMovementComponent.MaxWalkSpeed` (select `/Game/Enenmys/AI/Enums/E_MovmentSpeed` Speed :`NewEnumerator1` 100.0 :`NewEnumerator2` 600.0 :`NewEnumerator3` 1000.0 :!type "Float (single-precision)") (`self.CharacterMovement`)))
  (return _output_get))

(fn `UserConstructionScript`
  (`parent.UserConstructionScript`))