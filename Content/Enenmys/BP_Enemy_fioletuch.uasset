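; Purple enemy character with a ranged attack, built around a damage system component.
; Attack plays a sound and melee montage, spawns a bullet just ahead on montage notify, and signals attack end on completion or interruption.
; Damage triggers a hit sound; death hides the health bar, disables capsule collision and plays a capoeira montage before destroying the actor.
; SetMovmentSpeed maps movement states to walk speeds.
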(event `self.Attack`
  (`GameplayStatics.PlaySoundAtLocation` "/Game/EnemiesAssets/EnemiesModels/DaddyLongArms/fioletowyPojeb.fioletowyPojeb" (`self.K2_GetActorLocation`) (struct) 1.0 1.0 0.0 null null null null)
  (bind _notifyname (`|PlayMontage` (`self.Mesh`) "/Game/EnemiesAssets/EnemiesModels/DaddyLongArms/Standing_Melee_Attack_Backhand_montage.Standing_Melee_Attack_Backhand_montage")
    (:`OnCompleted`
      (`self.OnAttackEnd` :!label _label))
    (:`OnInterrupted`
      (goto _label))
    (:`OnNotifyBegin`
      (switch `name` _notifyname
        (:`throw`
          (`|SpawnActorFromClass` "/Game/FirstPerson/Blueprints/BP_Bullet_Mati_Oponent_Słabszy.BP_Bullet_Mati_Oponent_Słabszy_C" (`KismetMathLibrary.MakeTransform` (+ (* (`KismetMathLibrary.Normal` (`self.GetActorForwardVector`)) 50.0) (`self.K2_GetActorLocation`)) (`self.K2_GetActorRotation`)) "Undefined" "MultiplyWithRoot" null null))))))

(event `self.BPC_DamageSystem.OnDamageResponse`
  (params (DamageResponse :type "/Game/DamageSystem/E_DamageResponses Enum" :default "NewEnumerator0"))
  (`GameplayStatics.PlaySoundAtLocation` "/Game/EnemiesAssets/EnemiesModels/DaddyLongArms/bicieFioletowegoPojeba.bicieFioletowegoPojeba" (`self.K2_GetActorLocation`) (struct) 1.0 1.0 0.0 null null null null))

(event `self.BPC_DamageSystem.OnDeath`
  (`SceneComponent.SetVisibility` (`self.HealthBar`) false false)
  (`PrimitiveComponent.SetCollisionEnabled` (`self.CapsuleComponent`) "NoCollision")
  (`|PlayMontage` (`self.Mesh`) "/Game/EnemiesAssets/EnemiesModels/DaddyLongArms/Capoeira_Montage.Capoeira_Montage"
    (:`OnCompleted`
      (`self.K2_DestroyActor`))))

(fn `SetMovmentSpeed`
  (params (Speed :type "/Game/Enenmys/AI/Enums/E_MovmentSpeed Enum" :default "NewEnumerator0"))
  (returns (SpeedValue :type "Float (double-precision)"))
  (set `CharacterMovementComponent.MaxWalkSpeed` (select `/Game/Enenmys/AI/Enums/E_MovmentSpeed` Speed :`NewEnumerator1` 200.0 :`NewEnumerator2` 700.0 :`NewEnumerator3` 2000.0 :!type "Float (single-precision)") (`self.CharacterMovement`))
  (return 0.0))

(fn `UserConstructionScript`
  (`parent.UserConstructionScript`))